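; BP_Unit is a basic robot enemy unit, drawn as a Rumbeetle flipbook, that moves to requested destinations.
; MoveUnit compares destination X with its own to turn the actor left or right, then issues an AI move without pathfinding and shows the run flipbook.
; Tick restores the idle flipbook when the AI controller is idle.
; Non-looping playback restarts after random delays; velocity-based facing logic is left unconnected.
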(event `self.ReceiveBeginPlay`
  (bind _fb_rumbeetle (`self.FB_rumbeetle`))
  ;[1 1 1] Animation Control
  (`PaperFlipbookComponent.SetLooping` _fb_rumbeetle false)
  (`KismetSystemLibrary.Delay` (`KismetMathLibrary.RandomFloatInRange` 0.0 10.0))
  (`PaperFlipbookComponent.PlayFromStart` _fb_rumbeetle))

(event `self.FB_rumbeetle.OnFinishedPlaying`
  (bind _fb_rumbeetle (`self.FB_rumbeetle`))
  ;[1 1 1] Animation Control
  (`PaperFlipbookComponent.Stop` _fb_rumbeetle)
  (`KismetSystemLibrary.Delay` (`KismetMathLibrary.RandomFloatInRange` 0.0 10.0))
  (`PaperFlipbookComponent.PlayFromStart` _fb_rumbeetle))

(event `Moving Right`
  ;[1 1 1] Animation Control
  (`self.K2_SetActorRotation` (struct))
  (`PaperFlipbookComponent.SetFlipbook` (`self.FB_rumbeetle`) "/Game/GameFiles/Enemies/EnemyRobotBasic/Move/Flipbook_Rumbeetle_Run.Flipbook_Rumbeetle_Run"))

(event `Moving Left`
  ;[1 1 1] Animation Control
  (`self.K2_SetActorRotation` (struct :`Yaw` 180.0))
  (`PaperFlipbookComponent.SetFlipbook` (`self.FB_rumbeetle`) "/Game/GameFiles/Enemies/EnemyRobotBasic/Move/Flipbook_Rumbeetle_Run.Flipbook_Rumbeetle_Run"))

(event `Move Unit`
  (params (`Destination Vector` :type "Vector Structure"))
  (bind _returnvalue_x (`KismetMathLibrary.BreakVector2D` (`KismetMathLibrary.Conv_VectorToVector2D` `Destination Vector`)))
  (bind _returnvalue_x_2 (`KismetMathLibrary.BreakVector` (`self.K2_GetActorLocation` self)))
  (`/Engine/EditorBlueprintResources/StandardMacros.CompareFloat` _returnvalue_x _returnvalue_x_2
    (:`>`
      (`self.Moving Right`))
    (:`<`
      (`self.Moving Left`)))
  (`self.moveToLocation` `Destination Vector`))

(event `self.ReceiveTick`
  (params (DeltaSeconds :type "Float (single-precision)"))
  (bind _fb_rumbeetle (`self.FB_rumbeetle`))
  (bind _returnvalue (`AIController.GetMoveStatus` (`AIBlueprintHelperLibrary.GetAIController` self)))
  ;[1 1 1] Animation Control
  (bind _output_get (set `self.idle` (`|EnumEquality` _returnvalue "Idle")))
  (bind _output_get_2 (set `self.moving` (`|EnumEquality` _returnvalue "Moving")))
  (if _output_get
    (if (!= _fb_rumbeetle "/Game/GameFiles/Enemies/EnemyRobotBasic/idle/Flipbook_Rumbeetle_IdleIdle.Flipbook_Rumbeetle_IdleIdle")
      (`PaperFlipbookComponent.SetFlipbook` _fb_rumbeetle "/Game/GameFiles/Enemies/EnemyRobotBasic/idle/Flipbook_Rumbeetle_IdleIdle.Flipbook_Rumbeetle_IdleIdle"))
    (elif _output_get_2
      _)))

(fn `moveToLocation`
  (params (Destination :type "Vector Structure (by ref)"))
  (`PaperFlipbookComponent.SetFlipbook` (`self.FB_rumbeetle`) "/Game/GameFiles/Enemies/EnemyRobotBasic/Move/Flipbook_Rumbeetle_Run.Flipbook_Rumbeetle_Run")
  (`AIController.MoveToLocation` (`AIBlueprintHelperLibrary.GetAIController` self) Destination 5.0 false false false false null false))

(fn `UserConstructionScript`)