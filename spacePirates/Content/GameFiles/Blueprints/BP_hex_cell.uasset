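; BP_hex_cell is a clickable hex tile that reports clicks to the BP_hex_grid expected as its parent actor.
; Cursor hover swaps the SMHexCell material to a highlight and restores the basic material on exit.
; A click passes the cell's X and Y plus a Z derived from its scale to CellClicked, then applies a clicked material.
; That material is replaced when the cursor leaves, and a failed grid cast prints an error.
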(event `self.ReceiveActorOnClicked`
  (params (ButtonPressed :type "Key Structure"))
  (bind (_returnvalue_x _returnvalue_y _returnvalue_z) (`KismetMathLibrary.BreakVector` (`self.GetActorScale3D`)))
  (bind (_returnvalue_x_2 _returnvalue_y_2) (`KismetMathLibrary.BreakVector` (`self.K2_GetActorLocation`)))
  (bind _asbp_hex_grid (cast `/Game/GameFiles/Blueprints/BP_hex_grid` (`self.GetParentActor`))
    (:`then`
      (`/Game/GameFiles/Blueprints/BP_hex_grid.cell_clicked` _asbp_hex_grid (`KismetMathLibrary.MakeVector` _returnvalue_x_2 _returnvalue_y_2 (* 20.0 _returnvalue_z)))
      (`PrimitiveComponent.SetMaterial` (`self.SM_hex_cell`) 0 "/Engine/MapTemplates/Materials/BasicAsset03.BasicAsset03"))
    (:`CastFailed`
      (`KismetSystemLibrary.PrintString` "cast to grid failed" true true (struct :`G` 0.66 :`B` 1.0 :`A` 1.0) 100.0))))

(event `self.ReceiveActorBeginCursorOver`
  (`PrimitiveComponent.SetMaterial` (`self.SM_hex_cell`) 0 "/Engine/MapTemplates/Materials/BasicAsset01.BasicAsset01"))

(event `self.ReceiveActorEndCursorOver`
  (`PrimitiveComponent.SetMaterial` (`self.SM_hex_cell`) 0 "/Engine/BasicShapes/BasicShapeMaterial.BasicShapeMaterial"))

(fn `UserConstructionScript`)