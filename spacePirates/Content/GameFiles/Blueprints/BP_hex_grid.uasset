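; BP_hex_grid builds a grid of hex tiles as child actor components in its construction script.
; Nested loops over GridY and GridX space the tiles, shifting odd rows along X by Offset to form the hex layout.
; Each tile gets a random Z scale for varied height, re-rolled whenever construction reruns.
; Components, world XY positions and column/row indices are stored in parallel arrays; the event graph is inactive.
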(fn `UserConstructionScript`
  (for _index (range (+ (`self.Grid Y`) 1))
    (for _index_2 (range (+ (`self.Grid X`) 1))
      (bind _returnvalue (* _index_2 (`self.Spacing X`)))
      (bind _returnvalue_2 (* _index (`self.Spacing Y`)))
      (bind _returnvalue_3 (`AddComponent|NODE_AddChildActorComponent-0` :`RelativeTransform` (`KismetMathLibrary.MakeTransform` (`KismetMathLibrary.SelectVector` (`KismetMathLibrary.MakeVector` _returnvalue _returnvalue_2) (`KismetMathLibrary.MakeVector` (+ _returnvalue (`self.Offset`)) _returnvalue_2) (== (mod _index 2) 0)) (struct) (1.0 1.0 1.0))))
      (`SceneComponent.SetWorldScale3D` _returnvalue_3 (`KismetMathLibrary.MakeVector` 1.0 1.0 (`KismetMathLibrary.RandomFloatInRange` 1.0 3.0)))
      (`KismetArrayLibrary.Array_Add` (`self.hex_tiles`) _returnvalue_3)
      (bind (_returnvalue_x _returnvalue_y) (`KismetMathLibrary.BreakVector` (`SceneComponent.K2_GetComponentLocation` _returnvalue_3)))
      (`KismetArrayLibrary.Array_Add` (`self.hex_tile_coords`) (`KismetMathLibrary.MakeVector2D` _returnvalue_x _returnvalue_y))
      (`KismetArrayLibrary.Array_Add` (`self.hex_tile_index`) (`KismetMathLibrary.MakeVector2D` (`KismetMathLibrary.Conv_IntToDouble` _index_2) (`KismetMathLibrary.Conv_IntToDouble` _index))))))