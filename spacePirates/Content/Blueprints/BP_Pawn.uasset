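; Camera-style pawn that pans across world X and Y with the arrow keys or WASD.
; BeginPlay places it at a fixed position and rotation, sets the spring arm length and enables the mouse cursor and mouse-over events.
; Keys set direction flags, and Tick moves the pawn by a fixed frame-rate-dependent step.
; Nested branches allow one direction at a time, prioritized left, up, right, down.
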(event `self.ReceiveBeginPlay`
  (bind _returnvalue (`GameplayStatics.GetPlayerController` 0))
  (`self.K2_SetActorLocationAndRotation` (200.0 200.0 -40.0) (struct :`Pitch` -15.0 :`Yaw` 85.0))
  (set `PlayerController.bShowMouseCursor` true _returnvalue)
  (set `PlayerController.bEnableMouseOverEvents` true _returnvalue)
  (set `SpringArmComponent.TargetArmLength` 500.0 (`self.SpringArm`)))

(event `Key|Up`
  (params (Key :type "Key Structure"))
  (:`Pressed`
    (set `self.upArrow` true :!label _label))
  (:`Released`
    (set `self.upArrow` false :!label _label_2)))

(event `Key|W`
  (params (Key :type "Key Structure"))
  (:`Pressed`
    (goto _label))
  (:`Released`
    (goto _label_2)))

(event `Key|Right`
  (params (Key :type "Key Structure"))
  (:`Pressed`
    (set `self.rightArrow` true :!label _label_3))
  (:`Released`
    (set `self.rightArrow` false :!label _label_4)))

(event `Key|Left`
  (params (Key :type "Key Structure"))
  (:`Pressed`
    (set `self.leftArrow` true :!label _label_5))
  (:`Released`
    (set `self.leftArrow` false :!label _label_6)))

(event `Key|D`
  (params (Key :type "Key Structure"))
  (:`Pressed`
    (goto _label_3))
  (:`Released`
    (goto _label_4)))

(event `Key|A`
  (params (Key :type "Key Structure"))
  (:`Pressed`
    (goto _label_5))
  (:`Released`
    (goto _label_6)))

(event `Key|Down`
  (params (Key :type "Key Structure"))
  (:`Pressed`
    (set `self.downArrow` true :!label _label_7))
  (:`Released`
    (set `self.downArrow` false :!label _label_8)))

(event `self.ReceiveTick`
  (params (DeltaSeconds :type "Float (single-precision)"))
  (if (`self.leftArrow`)
    (`self.K2_AddActorWorldTransform` (`KismetMathLibrary.MakeTransform` (-50.0 0.0 0.0)))
    (elif (`self.upArrow`)
      (`self.K2_AddActorWorldTransform` (`KismetMathLibrary.MakeTransform` (0.0 50.0 0.0)))
      (elif (`self.rightArrow`)
        (`self.K2_AddActorWorldTransform` (`KismetMathLibrary.MakeTransform` (50.0 0.0 0.0)))
        (elif (`self.downArrow`)
          (`self.K2_AddActorWorldTransform` (`KismetMathLibrary.MakeTransform` (0.0 -50.0 0.0))))))))

(event `Key|S`
  (params (Key :type "Key Structure"))
  (:`Pressed`
    (goto _label_7))
  (:`Released`
    (goto _label_8)))

(fn `UserConstructionScript`)