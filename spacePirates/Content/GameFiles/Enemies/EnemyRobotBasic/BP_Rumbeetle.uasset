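; BP_Rumbeetle is a basic robot enemy with an animated sprite that can be sent to a location.
; Its sprite plays once, then replays after a random delay, starting from BeginPlay and repeating each time playback finishes.
; MoveUnit passes a destination to MoveToLocation, which issues a navmesh-projected move through the AI controller.
; Both steps print debug strings, and an AIMoveTo node is left unconnected.
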(event `self.ReceiveBeginPlay`
  (bind _sprite (`self.Sprite`))
  (`PaperFlipbookComponent.SetLooping` _sprite false)
  (`KismetSystemLibrary.Delay` (`KismetMathLibrary.RandomFloatInRange` 0.0 10.0))
  (`PaperFlipbookComponent.PlayFromStart` _sprite))

(event `Move Unit`
  (params (`Destination Vector` :type "Vector Structure"))
  (`self.moveToLocation` `Destination Vector`)
  (`KismetSystemLibrary.PrintString` (`KismetStringLibrary.Concat_StrStr` (`KismetSystemLibrary.GetDisplayName` self) (`KismetStringLibrary.Conv_VectorToString` `Destination Vector`))))

(event `self.Sprite.OnFinishedPlaying`
  (bind _sprite (`self.Sprite`))
  (`PaperFlipbookComponent.Stop` _sprite)
  (`KismetSystemLibrary.Delay` (`KismetMathLibrary.RandomFloatInRange` 0.0 10.0))
  (`PaperFlipbookComponent.PlayFromStart` _sprite))

(fn `moveToLocation`
  (params (Destination :type "Vector Structure (by ref)"))
  (bind _returnvalue (`AIController.MoveToLocation` (`AIBlueprintHelperLibrary.GetAIController` self) Destination 5.0 false true true true null true))
  (`KismetSystemLibrary.PrintString` (`|GetEnumeratorNameAsString` _returnvalue)))

(fn `UserConstructionScript`)