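; Game mode for a hex-grid unit game that spawns the grid and places units on random tiles at BeginPlay.
; On cell_clicked, recursive FindCellsInRange searches neighbours from the clicked cell, storing shorter paths per cell index within the first unit's MoveRange.
; A branch returns as soon as a path reaches that limit, skipping remaining neighbours.
; Results only feed debug prints; the MoveUnit call is disconnected.
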(event `self.ReceiveBeginPlay`
  (bind _returnvalue (`|SpawnActorFromClass` "/Game/GameFiles/Blueprints/BP_hex_grid.BP_hex_grid_C" (`KismetMathLibrary.MakeTransform` (0.0 0.0 0.0)) "AlwaysSpawn" "OverrideRootScale" self null))
  (set `self.Grid` _returnvalue)
  (for _ (range 1 (+ (`self.Unit Count`) 1))
    (bind _returnvalue_2 (`|SpawnActorFromClass` "/Game/GameFiles/Blueprints/BP_Unit.BP_Unit_C" (`KismetMathLibrary.MakeTransform` (`KismetArrayLibrary.Array_Random` (`/Game/GameFiles/Blueprints/BP_hex_grid.hex_tile_coords` _returnvalue))) "Undefined" "OverrideRootScale" null null))
    (`KismetArrayLibrary.Array_Add` (`self.Units`) _returnvalue_2)))

(event `cell_clicked`
  (params (`destination Vector` :type "Vector Structure"))
  (bind _possible_paths (`self.Possible Paths`))
  (bind _returnvalue (`KismetArrayLibrary.Array_Find` (`/Game/GameFiles/Blueprints/BP_hex_grid.hex_tile_coords` (`self.Grid`)) `destination Vector`))
  (bind _move_range (`/Game/GameFiles/Blueprints/BP_Unit.Move Range` (`|GetArrayItem` (`self.Units`))))
  (`BlueprintMapLibrary.Map_Clear` (`self.Possible Paths`))
  (bind _returnvalue_2 (`AddComponent|NODE_AddBP_PathfindingVectors-0` :`Possible Paths` (`|MakeArray` `destination Vector`)))
  (`BlueprintMapLibrary.Map_Add` _possible_paths _returnvalue _returnvalue_2)
  (bind (_movement_range _possibledestinationcells) (`self.FindCellsInRange` _move_range _returnvalue _possible_paths))
  (`KismetSystemLibrary.PrintString` (`KismetStringLibrary.BuildString_Int` "Length of PathList: " "" (`BlueprintMapLibrary.Map_Length` _possibledestinationcells)))
  (bind _values (`BlueprintMapLibrary.Map_Values` _possibledestinationcells))
  (for (_array_element _array_index) _values
    (bind _returnvalue_3 (`KismetArrayLibrary.Array_Length` (`/Game/GameFiles/Blueprints/BP_PathfindingVectors.Possible Paths` _array_element)))
    (`KismetSystemLibrary.PrintString` (`KismetStringLibrary.BuildString_Int` (`KismetStringLibrary.Conv_IntToString` _array_index) "Num of PathPoints: " _returnvalue_3))
    (if (> _returnvalue_3 _move_range)
      (`KismetSystemLibrary.PrintString` (`KismetStringLibrary.BuildString_Int` "too many points at" "" _array_index)))))

(fn `FindCellsInRange`
  (params (MovementRange :type "Integer (by ref)") (`Cell Index` :type Integer) (`Unit Location` :type "Map of Integer to /Game/GameFiles/Blueprints/BP_PathfindingVectors Object Reference (by ref)"))
  (returns (`Movement Range` :type Integer) (PossibleDestinationCells :type "Map of Integer to /Game/GameFiles/Blueprints/BP_PathfindingVectors Object Reference"))
  (bind _grid (`self.Grid`))
  (bind _possible_paths (`/Game/GameFiles/Blueprints/BP_PathfindingVectors.Possible Paths` (`BlueprintMapLibrary.Map_Find` `Unit Location` `Cell Index`)))
  (bind _values (`BlueprintMapLibrary.Map_Values` (`/Game/GameFiles/Blueprints/BP_hex_cell.adjacent cell indexes` (`|GetArrayItem` (`/Game/GameFiles/Blueprints/BP_hex_grid.hex_tiles` _grid) `Cell Index`))))
  (for _array_element _values
    (if (`KismetSystemLibrary.IsValid` _array_element)
      (bind _gridindex (`/Game/GameFiles/Blueprints/BP_hex_cell.gridIndex` _array_element))
      (if (`BlueprintMapLibrary.Map_Contains` `Unit Location` _gridindex)
        (if (< (+ (`KismetArrayLibrary.Array_Length` _possible_paths) 1) (`KismetArrayLibrary.Array_Length` (`/Game/GameFiles/Blueprints/BP_PathfindingVectors.Possible Paths` (`BlueprintMapLibrary.Map_Find` `Unit Location` _gridindex))))
          (bind _returnvalue (`AddComponent|NODE_AddBP_PathfindingVectors-1` :`Possible Paths` _possible_paths :!label _label))
          (bind _possible_paths_2 (`/Game/GameFiles/Blueprints/BP_PathfindingVectors.Possible Paths` _returnvalue))
          (`KismetArrayLibrary.Array_Add` _possible_paths_2 (`|GetArrayItem` (`/Game/GameFiles/Blueprints/BP_hex_grid.hex_tile_coords` _grid) _gridindex))
          (if (< (`KismetArrayLibrary.Array_Length` _possible_paths_2) MovementRange)
            (`BlueprintMapLibrary.Map_Add` `Unit Location` _gridindex _returnvalue)
            (`self.FindCellsInRange` MovementRange _gridindex `Unit Location`)
            (else
              (return MovementRange `Unit Location`))))
        (else
          (goto _label)))))
  (return MovementRange `Unit Location`))

(fn `UserConstructionScript`)