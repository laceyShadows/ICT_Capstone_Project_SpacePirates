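; Round orchestrator for a turn-based hex-grid game, cycling units through TurnOrder and notifying BP_GameMode as each phase starts.
; A FlipFlop alternates move and attack phases, advancing the unit index every second flip; a negative cell skips the phase.
; NextTurn steps along paths with delays, updates tile occupancy and removes killed units.
; Tick calls EndGame when a summed team-ID check indicates both teams are no longer alive.
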(event `Start Play`
  (bind _asbp_game_mode (cast `/Game/GameFiles/Blueprints/BP_GameMode` (`GameplayStatics.GetGameMode`) :!label _label))
  (`/Engine/EditorBlueprintResources/StandardMacros.IsValid` _asbp_game_mode
    (:`Is Valid`
      (`/Game/GameFiles/Blueprints/BP_GameMode.Unit Turn Start` _asbp_game_mode (`|GetArrayItem` (`self.Turn Order`) (`self.current_unit_index`))))))

(event `NextTurn`
  (params (movement_path :type "Array of Vector Structure (by ref)") (cell_index :type Integer))
  (bind _attacking_turn (`self.Attacking Turn`))
  (bind _turn_order (`self.Turn Order`))
  (bind _output (`|GetArrayItem` (`self.Turn Order`) (`self.current_unit_index`)))
  (if (< cell_index 0)
    (bind _isa (`/Engine/EditorBlueprintResources/StandardMacros.FlipFlop` :!label _label_2)
      (:`A`
        _)
      (:`B`
        (bind _result (`/Engine/EditorBlueprintResources/StandardMacros.IncrementInt` (`self.current_unit_index`))
          (:`  `
            (if (not (> (`KismetArrayLibrary.Array_Length` (`self.Turn Order`)) _result))
              (set `self.current_unit_index` 0))))))
    (set `self.Attacking Turn` _isa)
    (goto _label)
    (else
      (bind _element (`/Game/GameFiles/Blueprints/MacroLibrary.for_each_loop_with_delay` movement_path 0.3)
        (:`Loop Body`
          (if _attacking_turn
            (`/Game/GameFiles/Blueprints/BP_Unit.Attack` _output _element)
            (bind _asbp_game_mode (cast `/Game/GameFiles/Blueprints/BP_GameMode` (`GameplayStatics.GetGameMode`)))
            (`/Engine/EditorBlueprintResources/StandardMacros.IsValid` _asbp_game_mode
              (:`Is Valid`
                (set `/Game/GameFiles/Blueprints/BP_hex_cell.Occupied` false (`|GetArrayItem` (`/Game/GameFiles/Blueprints/BP_hex_grid.hex_tiles` (`/Game/GameFiles/Blueprints/BP_GameMode.Grid` _asbp_game_mode)) cell_index))))
            (else
              (bind (_prev_cell _current_cell) (`/Game/GameFiles/Blueprints/BP_Unit.Move Unit` _output _element cell_index))
              (bind _asbp_game_mode_2 (cast `/Game/GameFiles/Blueprints/BP_GameMode` (`GameplayStatics.GetGameMode`)))
              (`/Engine/EditorBlueprintResources/StandardMacros.IsValid` _asbp_game_mode_2
                (:`Is Valid`
                  (bind _hex_tiles (`/Game/GameFiles/Blueprints/BP_hex_grid.hex_tiles` (`/Game/GameFiles/Blueprints/BP_GameMode.Grid` _asbp_game_mode_2)))
                  (set `/Game/GameFiles/Blueprints/BP_hex_cell.Occupied` false (`|GetArrayItem` _hex_tiles _prev_cell))
                  (set `/Game/GameFiles/Blueprints/BP_hex_cell.Occupied` true (`|GetArrayItem` _hex_tiles _current_cell)))))))
        (:`Completed`
          (if _attacking_turn
            (`KismetSystemLibrary.Delay` 0.2)
            (for (_array_element _array_index) _turn_order
              (if (== cell_index (`/Game/GameFiles/Blueprints/BP_Unit.Current_Cell_Index` _array_element))
                (`/Game/GameFiles/Blueprints/BP_Unit.Killed` _array_element)
                (`KismetArrayLibrary.Array_Remove` _turn_order _array_index)
                (break)))
            (`KismetSystemLibrary.Delay` 3.0)
            (goto _label_2)
            (else
              (goto _label_2))))))))

(event `self.ReceiveTick`
  (params (DeltaSeconds :type "Float (single-precision)"))
  (bind _teams_alive (`self.Both Teams Alive`))
  (if (not _teams_alive)
    (bind _asbp_game_mode (cast `/Game/GameFiles/Blueprints/BP_GameMode` (`GameplayStatics.GetGameMode`)))
    (`/Engine/EditorBlueprintResources/StandardMacros.IsValid` _asbp_game_mode
      (:`Is Valid`
        (`/Game/GameFiles/Blueprints/BP_GameMode.End Game` _asbp_game_mode)))))

(fn `Both Teams Alive`
  (returns (`Teams Alive` :type Boolean))
  (locals (TeamCounter :type Integer))
  (for _array_element (`self.Turn Order`)
    (bind _team (`/Game/GameFiles/Blueprints/BP_Unit.Team` _array_element))
    (if (!= (`local.TeamCounter`) _team)
      (set `local.TeamCounter` (+ _team (`local.TeamCounter`)))))
  (if (> (`local.TeamCounter`) 3)
    (return true)
    (else
      (return false))))

(fn `UserConstructionScript`)